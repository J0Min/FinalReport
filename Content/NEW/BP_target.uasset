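; BP_target is a hittable target that flips down when its static mesh is struck and can be raised again.
; A hit on the mesh calls toDown and sets the IsHIt flag.
; An UP/Down enum guards toDown and toUp, so each acts only from the opposite state.
; A single timeline drives the mesh's relative pitch, playing from start to lower it and reversing from end to raise it.
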(event OnComponentHit(StaticMesh)
  (params (HitComponent :type Primitive%20Component%20Object%20Reference) (OtherActor :type Actor%20Object%20Reference) (OtherComp :type Primitive%20Component%20Object%20Reference) (NormalImpulse :type Vector :default "0, 0, 0") (Hit :type Hit%20Result%20Structure%20%28by%20ref%29))
  (CallFunction|ToDown)
  (Variables|Default|SetisHIt true))

(event Custom|toDown
  (switch Utilities|FlowControl|Switch|SwitchonstateEnum (Variables|Default|Getenum)
    (:NewEnumerator1
      (Variables|Default|Setenum "NewEnumerator2")
      (bind _rotation (Timeline|타임라인 PlayFromStart)
        (:Update
          (Transformation|SetRelativeRotation (Variables|Default|GetStaticMesh) (Math|Rotator|MakeRotator 0.0 _rotation 0.0) false false))))))

(event Custom|toUp
  (switch Utilities|FlowControl|Switch|SwitchonstateEnum (Variables|Default|Getenum)
    (:NewEnumerator2
      (Variables|Default|Setenum "NewEnumerator1")
      (bind _rotation (Timeline|타임라인 ReverseFromEnd)
        (:Update
          (Transformation|SetRelativeRotation (Variables|Default|GetStaticMesh) (Math|Rotator|MakeRotator 0.0 _rotation 0.0) false false))))))

(fn ConstructionScript)