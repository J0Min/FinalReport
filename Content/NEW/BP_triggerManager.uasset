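; BP_triggerManager is a level manager that links two trigger volumes, a set of BP_target actors and a door.
; The construction script gathers every BP_target in the level into the Target array.
; Overlapping Trig01 sets an enum state on all targets, and overlapping Trig02 calls ToUp on them.
; Tick ANDs every target's IsHIt flag and calls OpenDoor on each frame that all are hit.
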(event OnActorBeginOverlap(trig01)
  (params (OverlappedActor :type Actor%20Object%20Reference) (OtherActor :type Actor%20Object%20Reference))
  (for _array_element (Variables|Default|Gettarget)
    (Variables|/Game/NEW/BP_target.BP_target_C|Setenum _array_element "NewEnumerator1"))
  (Development|PrintString "Target Enabled"))

(event OnActorBeginOverlap(trig02)
  (params (OverlappedActor :type Actor%20Object%20Reference) (OtherActor :type Actor%20Object%20Reference))
  (for _array_element (Variables|Default|Gettarget)
    (Default|ToUp _array_element))
  (Development|PrintString "Target UP"))

(event EventBeginPlay)

(event Collision|EventActorBeginOverlap
  (params (OtherActor :type Actor%20Object%20Reference)))

(event EventTick
  (params (DeltaSeconds :type Float%20%28single-precision%29))
  (Variables|Default|SetisHIts true)
  (for _array_element (Variables|Default|Gettarget)
    (Variables|Default|SetisHIts (and (Variables|/Game/NEW/BP_target.BP_target_C|GetisHIt _array_element) (Variables|Default|GetisHIts))))
  (if (Variables|Default|GetisHIts)
    (Default|OpenDoor (Variables|Default|Getdoor))))

(fn ConstructionScript
  (bind _outactors (Actor|GetAllActorsOfClass "/Game/NEW/BP_target.BP_target_C"))
  (for (_array_element _array_index) _outactors
    (Utilities|Array|SetArrayElem (Variables|Default|Gettarget) _array_index _array_element true)))