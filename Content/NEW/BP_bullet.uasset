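; BP_bullet is a projectile actor that flies straight until it hits something, then removes itself.
; Each Tick, while IsHit is false, it moves with a swept local offset along the forward vector of the Arrow component's relative rotation, scaled by Speed without delta time.
; A hit on Sphere1 sets IsHit to stop the movement, then destroys the actor after a short delay through the Distroy function.
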(event OnComponentHit(Sphere1)
  (params (HitComponent :type Primitive%20Component%20Object%20Reference) (OtherActor :type Actor%20Object%20Reference) (OtherComp :type Primitive%20Component%20Object%20Reference) (NormalImpulse :type Vector :default "0, 0, 0") (Hit :type Hit%20Result%20Structure%20%28by%20ref%29))
  (Variables|Default|SetisHit true)
  (Utilities|FlowControl|Delay 2.0)
  (CallFunction|Distroy))

(event EventBeginPlay)

(event Collision|EventActorBeginOverlap
  (params (OtherActor :type Actor%20Object%20Reference)))

(event EventTick
  (params (DeltaSeconds :type Float%20%28single-precision%29))
  (if (not (Variables|Default|GetisHit))
    (Transformation|AddActorLocalOffset (* (Math|Vector|GetForwardVector (Variables|/Script/Engine.SceneComponent|GetRelativeRotation (Variables|Default|GetArrow))) (Variables|Default|GetSpeed)) true false)))

(fn ConstructionScript)

(fn Distroy
  (Actor|DestroyActor))